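; BP_ExplodeAttacker is a movable pawn that attacks by exploding and also sets off an explosion when it dies.
; Unnamed requests resolve to the explode attack command for enemy targets and to the move command otherwise.
; The construction script binds the death event on authority only.
; Unless the pawn is invincible, that handler strips defense, restores minimal health, flags death to be skipped and issues itself an Explode request at its location.
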(event Custom|Event%20OnPawnDied
  (params (DiedPawn :type PF%20Pawn%20Object%20Reference))
  (if (not (Class|PFPawn|IsInvincible DiedPawn))
    (Variables|Default|SetDefense 0)
    (Variables|Default|SetCurrentHealth 1)
    (Variables|Default|SetbShouldSkipDied true)
    (Class|ConsciousPawn|Receive (Utilities|Struct|MakeTargetRequest "Explode" 0 (Transformation|GetActorLocation)))))

(event EventBeginPlay)

(event Collision|EventActorBeginOverlap
  (params (OtherActor :type Actor%20Object%20Reference)))

(event EventTick
  (params (DeltaSeconds :type Float%20%28single-precision%29)))

(fn ConstructionScript
  (Networking|SwitchHasAuthority
    (:Authority
      (EventDispatchers|BindEventtoOnPawnDied (EventDispatchers|CreateEvent :!event Custom|Event%20OnPawnDied)))))

(fn ResolveRequestWithoutName
  (params (Request :type Target%20Request%20Structure%20%28by%20ref%29))
  (if (Utilities|Enum|Equal(Enum) (Class|PFPawn|GetPawnRole (.TargetPawn (Utilities|Struct|BreakTargetRequest Request))) "Enemy")
    (return (Variables|Default|GetExplodeAttackCommand))
    (else
      (return (Variables|Default|GetMoveCommandComponent)))))