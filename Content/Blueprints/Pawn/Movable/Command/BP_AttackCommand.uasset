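; BP_AttackCommand is a pawn command that performs an attack on the request's target pawn.
; On execution it briefly doubles the executing pawn's scale as simple attack feedback, then restores it after a short delay.
; It then applies damage based on the pawn's Attack stat, credited to the executing controller and pawn, and ends the command as a success.
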(event EventBeginPlay)

(event EventTick
  (params (DeltaSeconds :type Float%20%28single-precision%29)))

(event EventInternalBeginExecute
  (bind _returnvalue (Class|CommandComponent|GetExecutePawn))
  (Transformation|SetActorScale3D _returnvalue "2.000000,2.000000,2.000000")
  (Utilities|FlowControl|Delay 0.2)
  (Transformation|SetActorScale3D _returnvalue "1.000000,1.000000,1.000000")
  (Game|Damage|ApplyDamage (.TargetPawn (Utilities|Struct|BreakTargetRequest (Class|CommandComponent|GetRequest))) (Math|Conversions|ToFloat(Integer) (Variables|/Script/Pathfinding.PFPawn|GetAttack _returnvalue)) (Class|CommandComponent|GetExecuteController) _returnvalue "/Script/Engine.DamageType")
  (Class|CommandComponent|EndExecute "Success"))