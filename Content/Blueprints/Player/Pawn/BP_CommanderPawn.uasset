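; BP_CommanderPawn is the commander player pawn, with a flag-material mesh and logic for spawning BP_PFPawn units.
; BeginPlay enables input for player 0, the Test event spawns a unit at the pawn's location, and Tick does nothing.
; The construction script creates a dynamic M_PFPawnFlag material on the mesh.
; Unconnected graph logic would tint the mesh with the player state's color and spawn units where a mouse-cursor trace hits.
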(event EventBeginPlay
  (Input|EnableInput (Game|GetPlayerController 0)))

(event Collision|EventActorBeginOverlap
  (params (OtherActor :type Actor%20Object%20Reference)))

(event EventTick
  (params (DeltaSeconds :type Float%20%28single-precision%29))
  (Utilities|FlowControl|Sequence))

(event EventTest
  (Class|CommanderPawn|SpawnPFPawn "/Game/Blueprints/Player/Pawn/BP_PFPawn.BP_PFPawn_C" (Transformation|GetActorLocation)))

(fn ConstructionScript
  (Class|PFBlueprintFunctionLibrary|CreateDynamicMaterialInstanceforStaticMesh (Variables|Default|GetStaticMesh) "/Game/Art/Materials/M_PFPawnFlag.M_PFPawnFlag"))